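; BP_TestGameInstance is a test game instance that handles creating and joining online multiplayer sessions.
; CreateSession destroys any existing session, then creates an Advanced Sessions session with the caller's settings and the server name stored as an extra property.
; On success it hides the mouse cursor and opens L_Test as a listen server.
; JoinSession joins a given search result and hides the cursor on success.
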(event `CreateSession`
  (params (PublicConnections :type Integer) (PrivateConnections :type Integer) (UseLan :type Boolean) (bAllowInvites :type Boolean :default true) (bIsDedicatedServer :type Boolean) (bUsePresence :type Boolean :default true) (bUseLobbiesIfAvailable :type Boolean :default true) (bAllowJoinViaPresence :type Boolean :default true) (bAllowJoinViaPresenceFriendsOnly :type Boolean) (bAntiCheatProtected :type Boolean) (bUsesStats :type Boolean) (bShouldAdvertise :type Boolean :default true) (bUseLobbiesVoiceChatIfAvailable :type Boolean) (bStartAfterCreate :type Boolean :default true) (ServerName :type String))
  (bind _returnvalue (`GameplayStatics.GetPlayerController` 0))
  (`DestroySessionCallbackProxy.DestroySession` _returnvalue
    (:`then`
      (`CreateSessionCallbackProxyAdvanced.CreateAdvancedSession` (`|MakeArray` (`AdvancedSessionsLibrary.MakeLiteralSessionPropertyString` "ServerName" ServerName)) _returnvalue PublicConnections PrivateConnections UseLan bAllowInvites bIsDedicatedServer bUsePresence bUseLobbiesIfAvailable bAllowJoinViaPresence bAllowJoinViaPresenceFriendsOnly bAntiCheatProtected bUsesStats bShouldAdvertise bUseLobbiesVoiceChatIfAvailable bStartAfterCreate
        (:`OnSuccess`
          (set `PlayerController.bShowMouseCursor` false (`GameplayStatics.GetPlayerController` 0))
          (`GameplayStatics.OpenLevel` "L_Test" false "listen"))))))

(event `JoinSession`
  (params (SearchResult :type "BlueprintSessionResult Structure (by ref)"))
  (bind _returnvalue (`GameplayStatics.GetPlayerController` 0))
  (`JoinSessionCallbackProxy.JoinSession` _returnvalue SearchResult
    (:`OnSuccess`
      (set `PlayerController.bShowMouseCursor` false _returnvalue))))