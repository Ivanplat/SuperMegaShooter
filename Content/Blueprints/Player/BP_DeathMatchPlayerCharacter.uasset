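; Player character Blueprint for deathmatch that adds a debug-style score readout.
; Pressing Tab casts the PlayerState to CPP_PlayerState and prints kills and deaths as a "K/D" text.
; A disconnected print of the inventory component's main, secondary, melee and selected weapons never runs, and the construction script is empty.
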(event `Key|Tab`
  (params (Key :type "Key Structure"))
  (bind _ascpp_player_state (cast `CPP_PlayerState` (`self.PlayerState`) :!pure true))
  (:`Pressed`
    (`KismetSystemLibrary.PrintText` (`|FormatText` "{K}/{D}" (`CPP_PlayerState.GetKills` _ascpp_player_state) (`CPP_PlayerState.GetDeaths` _ascpp_player_state)))))

(fn `UserConstructionScript`)