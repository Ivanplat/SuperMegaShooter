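; Test game instance Blueprint that handles hosting and joining multiplayer sessions through Advanced Sessions nodes.
; CreateSession calls DestroySession, continues without waiting for its result, creates a session with optional LAN, then opens L_TestLevel as a listen server.
; Its PublicConnections input is unused, while private connections are hardcoded.
; JoinSession joins a given search result, hiding the cursor on success or printing an error on failure.
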(event `CreateSession`
  (params (PublicConnections :type Integer) (UseLan :type Boolean))
  (bind _returnvalue (`GameplayStatics.GetPlayerController` 0))
  (`DestroySessionCallbackProxy.DestroySession` _returnvalue
    (:`then`
      (`CreateSessionCallbackProxyAdvanced.CreateAdvancedSession` (`|MakeArray` (struct) :!type "SessionPropertyKeyPair Structure") _returnvalue 100 20 UseLan true false true true true true false true
        (:`OnSuccess`
          (set `PlayerController.bShowMouseCursor` false (`GameplayStatics.GetPlayerController` 0))
          (`GameplayStatics.OpenLevelBySoftObjectPtr` "/Game/Maps/L_TestLevel.L_TestLevel" false "listen"))))))

(event `JoinSession`
  (params (SearchResult :type "BlueprintSessionResult Structure (by ref)"))
  (bind _returnvalue (`GameplayStatics.GetPlayerController` 0))
  (`JoinSessionCallbackProxy.JoinSession` _returnvalue SearchResult
    (:`OnSuccess`
      (set `PlayerController.bShowMouseCursor` false _returnvalue))
    (:`OnFailure`
      (`KismetSystemLibrary.PrintString` "UNABLE TO CONNECT"))))